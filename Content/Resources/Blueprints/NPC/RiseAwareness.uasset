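; Behavior tree task that raises a Knight NPC's awareness based on blackboard distance to its target.
; Within a tenth of max sight distance, awareness jumps to full; farther out, it grows by a clamped inverse-distance term scaled by AwarenessFactor.
; It writes the blackboard, then recomputes for the Knight's variable, leaving that one increment ahead outside close range.
; It prints the blackboard value and finishes successfully, but never finishes if the Knight cast fails.
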(event `self.ReceiveExecuteAI`
  (params (OwnerController :type "AIController Object Reference") (ControlledPawn :type "Pawn Object Reference"))
  (bind _awareness (`self.Awareness`))
  (bind _returnvalue (`BTFunctionLibrary.GetBlackboardValueAsFloat` (`self.MaxSightDistance`)))
  (bind _returnvalue_2 (`BTFunctionLibrary.GetBlackboardValueAsFloat` (`self.CurrentDistance`)))
  (bind _returnvalue_3 (`BTFunctionLibrary.GetBlackboardValueAsFloat` _awareness))
  (bind _returnvalue_4 (* _returnvalue 0.1))
  (bind _returnvalue_5 (+ _returnvalue_3 (* (`KismetMathLibrary.FClamp` (/ (* _returnvalue 0.9) (- _returnvalue_2 _returnvalue_4)) 1.0 100.0) (`self.AwarenessFactor`))))
  (bind _asknight (cast `/Game/Resources/Blueprints/NPC/Knight` ControlledPawn))
  (if (< _returnvalue_2 _returnvalue_4)
    (`BTFunctionLibrary.SetBlackboardValueAsFloat` _awareness 100.0)
    (set `/Game/Resources/Blueprints/NPC/Knight.Awareness` 100.0 _asknight)
    (else
      (`BTFunctionLibrary.SetBlackboardValueAsFloat` _awareness _returnvalue_5)
      (set `/Game/Resources/Blueprints/NPC/Knight.Awareness` _returnvalue_5 _asknight)))
  (`KismetSystemLibrary.PrintString` (`KismetStringLibrary.Conv_DoubleToString` _returnvalue_3))
  (`self.FinishExecute` true))