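; Behavior Tree task that records the player's last seen location on the Blackboard for NPC AI.
; While SeeingPlayer is true, it writes the player capsule's location to PlayerLastSeenLocation.
; When sight is lost, a timer handle is meant to extend updates briefly, though this graph never starts that timer, only checks, clears or unpauses it.
; The task always finishes successfully in the same execution.
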(event `self.ReceiveExecuteAI`
  (params (OwnerController :type "AIController Object Reference") (ControlledPawn :type "Pawn Object Reference"))
  (bind _timer (`self.Timer`))
  (bind _returnvalue (`SceneComponent.K2_GetComponentLocation` (`Character.CapsuleComponent` (`GameplayStatics.GetPlayerCharacter` 0))))
  ;[1 1 1] 如果玩家刚脱离视野，就继续延长0.5-1s的位置获取
  (if (`BTFunctionLibrary.GetBlackboardValueAsBool` (`self.SeeingPlayer`))
    (bind _output_get (set `self.Player Last Location` _returnvalue))
    (`BTFunctionLibrary.SetBlackboardValueAsVector` (`self.PlayerLastSeenLocation`) _output_get)
    (elif (`KismetSystemLibrary.K2_IsValidTimerHandle` _timer)
      (bind _output_get_2 (set `self.Player Last Location` _returnvalue))
      (`BTFunctionLibrary.SetBlackboardValueAsVector` (`self.PlayerLastSeenLocation`) _output_get_2)
      (if (<= (`KismetSystemLibrary.K2_GetTimerElapsedTimeHandle` _timer) (`self.RemainingTime`))
        (`KismetSystemLibrary.K2_ClearAndInvalidateTimerHandle` _timer))
      (else
        (`KismetSystemLibrary.K2_UnPauseTimerHandle` _timer))))
  (`self.FinishExecute` true))