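; AI controller for Knight enemies that detects the player and drives alert states from patrol to aggression.
; It runs Enemy_BT and feeds the blackboard sight, noise locations and the player's last known position from AI Perception and tracking.
; Tick switches the pawn's state using an awareness meter that fills faster at closer range, instantly when very near.
; A timer briefly extends tracking after losing sight and times out searches.
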(event `self.ReceiveTick`
  (params (DeltaSeconds :type "Float (single-precision)"))
  (bind _mypawn (`self.MyPawn`))
  (bind _awareness (`/Game/Resources/Blueprints/NPC/Knight.Awareness` (`self.MyPawn`)))
  (bind _returnvalue (>= _awareness 100.0))
  (if (> (`/Game/Resources/Blueprints/NPC/Knight.Awareness` _mypawn) 0.0)
    (set `/Game/Resources/Blueprints/NPC/Knight.ShowABar` true _mypawn)
    (else
      (set `/Game/Resources/Blueprints/NPC/Knight.ShowABar` false _mypawn)))
  (`self.CalculateCurrentDist`)
  (switch `/Game/Resources/Blueprints/AI_State` (`/Game/Resources/Blueprints/NPC/Knight.State` (`self.MyPawn`))
    (:`NewEnumerator0`
      (if (< _awareness 50.0)
        (if (`self.SeeingPlayer`)
          (`self.RaiseAwareness`)
          (else
            (`self.DecreaseAwareness`)))
        (else
          (`self.ChangeState` "NewEnumerator1"))))
    (:`NewEnumerator1`
      (if (`self.SeeingPlayer`)
        (`self.RaiseAwareness`)
        (if _returnvalue
          (`self.ChangeState` "NewEnumerator2"))
        (elif _returnvalue
          (`self.ChangeState` "NewEnumerator2")
          (else
            (`self.ChangeState` "NewEnumerator9")))))
    (:`NewEnumerator2`
      (`self.GetPlayerLastLocation`)
      (`self.ClearAwareness`))
    (:`NewEnumerator4`
      (if (`self.SeeingPlayer`)
        (`self.RaiseAwareness`)
        (if _returnvalue
          (`self.ChangeState` "NewEnumerator2"))))
    (:`NewEnumerator3`
      (if (`self.SeeingPlayer`)
        (`self.RaiseAwareness`)
        (if _returnvalue
          (`self.ChangeState` "NewEnumerator2"))
        (else
          (`self.StartTimer`)
          (if (>= (`KismetSystemLibrary.K2_GetTimerElapsedTimeHandle` (`self.Timer`)) (`self.SearchingTime`))
            (`self.StopTimer`)
            (`self.ChangeState` "NewEnumerator0")))))
    (:`NewEnumerator8`
      (`MovementComponent.StopMovementImmediately` (`Character.CharacterMovement` (`self.MyPawn`))))
    (:`NewEnumerator9`
      (if (`self.SeeingPlayer`)
        (`self.RaiseAwareness`)
        (if _returnvalue
          (`self.ChangeState` "NewEnumerator2"))))))

(event `self.ReceiveBeginPlay`
  (`self.RunBehaviorTree` "/Game/Resources/Blueprints/NPC/Enemy_BT.Enemy_BT")
  (bind _asknight (cast `/Game/Resources/Blueprints/NPC/Knight` (`self.K2_GetPawn`)))
  (bind _output_get (set `self.MyPawn` _asknight))
  (`/Game/Resources/Blueprints/NPC/Knight.On State Changed` _output_get)
  (`BlackboardComponent.SetValueAsFloat` (`AIBlueprintHelperLibrary.GetBlackboard` null) "MaxSightDistance" (`self.MaxSightDistance`) :!pinned true) ; Should be changed based on perception value.
)

(event `self.AIPerception.OnTargetPerceptionUpdated`
  (params (Actor :type "Actor Object Reference") (Stimulus :type "AIStimulus Structure"))
  (bind _returnvalue (`AIBlueprintHelperLibrary.GetBlackboard` null))
  ;[1 1 1] 视觉感知
  (cast `/Game/Resources/Blueprints/Player` Actor)
  (if (`.bSuccessfullySensed` (break `AIStimulus` Stimulus))
    (`BlackboardComponent.SetValueAsBool` _returnvalue "SeeingPlayer" true)
    (set `self.SeeingPlayer` true)
    (else
      (`KismetSystemLibrary.PrintString` "Cannot see" true true (struct :`R` 1.0 :`G` 0.910763 :`A` 1.0) 10.0)
      (`BlackboardComponent.SetValueAsBool` _returnvalue "SeeingPlayer" false)
      (set `self.SeeingPlayer` false))))

(event `self.AIPerception.OnPerceptionUpdated`
  (params (UpdatedActors :type "Array of Actor Object Reference (by ref)"))
  (bind _state (`/Game/Resources/Blueprints/NPC/Knight.State` (`self.MyPawn`)))
  ;[1 1 1] 听觉
  (if (`|EnumEquality` _state "NewEnumerator6")
    _
    (elif (not (`|EnumEquality` _state "NewEnumerator5"))
      (for _array_element UpdatedActors
        (bind _info (`AIPerceptionComponent.GetActorsPerception` (`self.AIPerception`) _array_element))
        (for _array_element_2 (`.LastSensedStimuli` (break `ActorPerceptionBlueprintInfo` _info))
          (bind (_age _expirationage _strength _stimuluslocation _receiverlocation _tag) (break `AIStimulus` _array_element_2))
          (if (== _tag "Noise") :!pinned true
            (`BlackboardComponent.SetValueAsVector` (`AIBlueprintHelperLibrary.GetBlackboard` null) "LastHearLocation" _stimuluslocation)))))))

(fn `CalculateCurrentDist`
  (bind _maxsightdistance (`self.MaxSightDistance`))
  (set `self.CurrentDistance` (`KismetMathLibrary.FClamp` (`KismetMathLibrary.Vector_Distance` (`self.K2_GetActorLocation` (`self.MyPawn`)) (`self.K2_GetActorLocation` (`GameplayStatics.GetPlayerPawn` 0))) (* _maxsightdistance 0.1) _maxsightdistance)))

(fn `ChangeState`
  (params (State :type "/Game/Resources/Blueprints/AI_State Enum" :default "NewEnumerator0"))
  (bind _mypawn (`self.MyPawn`))
  (set `/Game/Resources/Blueprints/NPC/Knight.State` (`local.State`) _mypawn)
  (`/Game/Resources/Blueprints/NPC/Knight.On State Changed` _mypawn))

(fn `ClearAwareness`
  (set `/Game/Resources/Blueprints/NPC/Knight.Awareness` 0.0 (`self.MyPawn`))
  (`BlackboardComponent.SetValueAsFloat` (`self.Blackboard`) "Awareness" 0.0))

(fn `DecreaseAwareness`
  (bind _mypawn (`self.MyPawn`))
  (set `/Game/Resources/Blueprints/NPC/Knight.Awareness` (- (`/Game/Resources/Blueprints/NPC/Knight.Awareness` _mypawn) (`self.AwareDecreSpeed`)) _mypawn))

(fn `GetPlayerLastLocation`
  (bind _timer (`self.Timer`))
  (bind _blackboard (`self.Blackboard`))
  (bind _returnvalue (`SceneComponent.K2_GetComponentLocation` (`Character.CapsuleComponent` (`GameplayStatics.GetPlayerCharacter` 0))))
  ;[1 1 1] 如果玩家刚脱离视野，就继续延长0.5-1s的位置获取
  (if (`self.SeeingPlayer`)
    (bind _output_get (set `self.Player Last Location` _returnvalue))
    (`BlackboardComponent.SetValueAsVector` _blackboard "PlayerLastLocation" _output_get)
    (else
      (`self.StartTimer`)
      (if (<= (`KismetSystemLibrary.K2_GetTimerElapsedTimeHandle` _timer) (`self.RemainingTime`))
        (bind _output_get_2 (set `self.Player Last Location` _returnvalue))
        (`BlackboardComponent.SetValueAsVector` _blackboard "PlayerLastLocation" _output_get_2)
        (else
          (`KismetSystemLibrary.K2_ClearAndInvalidateTimerHandle` _timer)
          (`self.ChangeState` "NewEnumerator4"))))))

(fn `RaiseAwareness`
  (bind _blackboard (`self.Blackboard`))
  (bind _returnvalue (* (`self.MaxSightDistance`) (`self.DistanceFactor`)))
  (bind _returnvalue_2 (+ (`BlackboardComponent.GetValueAsFloat` _blackboard "Awareness") (* (`KismetMathLibrary.FClamp` (/ (* (`self.MaxSightDistance`) (- 1.0 (`self.DistanceFactor`))) (- (`self.CurrentDistance`) _returnvalue)) 1.0 100.0) (`self.AwarenessFactor`))))
  (if (< (`self.CurrentDistance`) _returnvalue)
    (`BlackboardComponent.SetValueAsFloat` _blackboard "Awareness" 100.0)
    (set `/Game/Resources/Blueprints/NPC/Knight.Awareness` 100.0 (`self.MyPawn`))
    (else
      (`BlackboardComponent.SetValueAsFloat` _blackboard "Awareness" _returnvalue_2)
      (set `/Game/Resources/Blueprints/NPC/Knight.Awareness` _returnvalue_2 (`self.MyPawn`)))))

(fn `StartTimer`
  (if (not (`KismetSystemLibrary.K2_IsValidTimerHandle` (`self.Timer`)))
    (bind _returnvalue (`KismetSystemLibrary.K2_SetTimer` self "StartTimer" (`self.SearchingTime`)))
    (bind _output_get (set `self.Timer` _returnvalue))
    (`KismetSystemLibrary.K2_UnPauseTimerHandle` _output_get)
    (`KismetSystemLibrary.PrintString` "Start Timing.")))

(fn `StopTimer`
  (`KismetSystemLibrary.K2_ClearAndInvalidateTimerHandle` (`self.Timer`))
  (`KismetSystemLibrary.PrintString` "Stop timing"))

(fn `UserConstructionScript`)