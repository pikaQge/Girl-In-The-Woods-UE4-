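; BP_Elevator is a machine actor that moves vertically when activated and returns when inactivated.
; It caches its root's world location on BeginPlay as the base position.
; ActivateMachine plays a timeline that lerps a Z offset between Low and Hight, setting the actor location relative to that base.
; InactivateMachine reverses the same timeline to move it back.
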(event `self.ReceiveBeginPlay`
  (set `self.location` (`SceneComponent.K2_GetComponentLocation` (`self.DefaultSceneRoot`))))

(event `self.ActivateMachine`
  (bind (_location_x _location_y _location_z) (`KismetMathLibrary.BreakVector` (`self.location`)))
  (bind (_direction _newtrack_0) (`Timeline|时间轴_0` :!label _label)
    (:`Update`
      (`self.K2_SetActorLocation` (`KismetMathLibrary.MakeVector` _location_x _location_y (+ (`KismetMathLibrary.Lerp` (`self.low`) (`self.hight`) _newtrack_0) _location_z))))))

(event `self.InactivateMachine`
  (goto _label :!via `Reverse`))

(fn `UserConstructionScript`)