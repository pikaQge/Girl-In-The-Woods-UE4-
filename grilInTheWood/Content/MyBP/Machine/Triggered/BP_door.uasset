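; Triggered door machine that swings open when activated and closes when inactivated.
; ActivateMachine plays a timeline and InactivateMachine reverses it, lerping a yaw offset on the Door component toward an open angle.
; The offset is added to the root's world rotation cached at BeginPlay, and the sum is applied as the Door's relative rotation.
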(event `self.ReceiveBeginPlay`
  (set `self.rotation` (`SceneComponent.K2_GetComponentRotation` (`self.DefaultSceneRoot`))))

(event `self.ActivateMachine`
  (bind (_rotation_roll _rotation_pitch _rotation_yaw) (`KismetMathLibrary.BreakRotator` (`self.rotation`)))
  (bind (_direction `_新建轨道_0`) (`Timeline|时间轴_0` :!label _label)
    (:`Update`
      (`SceneComponent.K2_SetRelativeRotation` (`self.door`) (`KismetMathLibrary.MakeRotator` _rotation_roll _rotation_pitch (+ (`KismetMathLibrary.Lerp` 0.0 100.0 `_新建轨道_0`) _rotation_yaw)) false false))))

(event `self.InactivateMachine`
  (goto _label :!via `Reverse`))

(fn `UserConstructionScript`)