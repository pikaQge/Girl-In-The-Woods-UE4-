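; Behavior tree task that finds the current patrol point for a Knight NPC.
; It reads the PathIndex blackboard value, takes that entry from the Knight's PatrolPath points and transforms it from the path actor's local space to world space.
; The result is written to the PatrolPoint key and the task succeeds; a failed cast or invalid path never calls FinishExecute.
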(event `self.ReceiveExecuteAI`
  (params (OwnerController :type "AIController Object Reference") (ControlledPawn :type "Pawn Object Reference"))
  (bind _asknight (cast `/Game/Resources/Blueprints/NPC/Knight` ControlledPawn))
  (bind _patrolpath (`/Game/Resources/Blueprints/NPC/Knight.PatrolPath` _asknight) ; Get PatrolPath of Enemy Character
    (:`then`
      (`BTFunctionLibrary.SetBlackboardValueAsVector` (`self.PatrolPoint`) (`KismetMathLibrary.TransformLocation` (`Actor.GetTransform` _patrolpath) (`|GetArrayItem` (`/Game/MyBP/AI/PatrolPath.patrolPoints` _patrolpath) (`BTFunctionLibrary.GetBlackboardValueAsInt` (`self.PathIndex`)))))
      (`self.FinishExecute` true))
    (:`else`)))