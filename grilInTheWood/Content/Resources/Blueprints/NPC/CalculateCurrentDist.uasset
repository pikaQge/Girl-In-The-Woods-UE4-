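; Behavior tree task for NPC AI that calculates the current distance between a target and an enemy location.
; On execution it reads both location vectors from the blackboard and measures the distance between them.
; It clamps the result between one tenth of the blackboard's max sight distance and the full value.
; The clamped float is written to the CurrentDistance key, and the task immediately finishes successfully.
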(event `self.ReceiveExecuteAI`
  (params (OwnerController :type "AIController Object Reference") (ControlledPawn :type "Pawn Object Reference"))
  (bind _returnvalue (`BTFunctionLibrary.GetBlackboardValueAsFloat` (`self.MaxSightDistance`)))
  (`BTFunctionLibrary.SetBlackboardValueAsFloat` (make `BlackboardKeySelector` _ "CurrentDistance") (`KismetMathLibrary.FClamp` (`KismetMathLibrary.Vector_Distance` (`BTFunctionLibrary.GetBlackboardValueAsVector` (`self.TargetLocation`)) (`BTFunctionLibrary.GetBlackboardValueAsVector` (`self.EnemyLocation`))) (* _returnvalue 0.1) _returnvalue))
  (`self.FinishExecute` true))