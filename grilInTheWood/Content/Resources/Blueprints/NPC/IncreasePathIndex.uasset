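; Behavior tree task that advances a Knight NPC to the next point on its patrol path.
; On execute it increments the PathIndex blackboard value, wrapping to zero after the last PatrolPoints entry, then finishes successfully.
; A disconnected, never-run branch searches for the patrol point nearest the Knight but writes a constant zero to NearestPointIndex instead of the found index.
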(event `self.ReceiveExecuteAI`
  (params (OwnerController :type "AIController Object Reference") (ControlledPawn :type "Pawn Object Reference"))
  (bind _returnvalue (`BTFunctionLibrary.GetBlackboardValueAsInt` (`self.PathIndex`)))
  (bind _asknight (cast `/Game/Resources/Blueprints/NPC/Knight` ControlledPawn))
  (if (== _returnvalue (- (`KismetArrayLibrary.Array_Length` (`/Game/MyBP/AI/PatrolPath.patrolPoints` (`/Game/Resources/Blueprints/NPC/Knight.PatrolPath` _asknight))) 1))
    (`BTFunctionLibrary.SetBlackboardValueAsInt` (`self.PathIndex`))
    (else
      (bind _result (`/Engine/EditorBlueprintResources/StandardMacros.IncrementInt` _returnvalue)
        (:`  `
          (`BTFunctionLibrary.SetBlackboardValueAsInt` (`self.PathIndex`) _result)))))
  (`self.FinishExecute` true))