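; Knight enemy NPC character with an awareness bar, fireball knockback, blinding, and fainting with revival.
; State changes are pushed to the AI Blackboard's State key, while a toggle controls the awareness widget's ticking.
; Faint ragdolls the mesh and disables movement; Revive reattaches it to the capsule and restores walking.
; Tick snaps the capsule to the mesh's XY in one state and draws debug capsule and forward head trace.
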(event `self.ReceiveTick`
  (params (DeltaSeconds :type "Float (single-precision)"))
  (bind _awarenessbar (`self.AwarenessBar`))
  (bind _capsulecomponent (`self.CapsuleComponent`))
  (bind (_returnvalue_x _returnvalue_y) (`KismetMathLibrary.BreakVector` (`SceneComponent.K2_GetComponentLocation` (`self.Mesh`))))
  (bind (_returnvalue_x_2 _returnvalue_y_2 _returnvalue_z) (`KismetMathLibrary.BreakVector` (`SceneComponent.K2_GetComponentLocation` _capsulecomponent)))
  (bind _returnvalue (`SceneComponent.GetSocketLocation` (`self.Mesh`) "head"))
  (bind (_returnvalue_x_3 _returnvalue_y_3 _returnvalue_z_2) (`KismetMathLibrary.BreakVector` (`KismetMathLibrary.GetForwardVector` (`self.K2_GetActorRotation`))))
  (`KismetSystemLibrary.DrawDebugCapsule` (`SceneComponent.K2_GetComponentLocation` _capsulecomponent) 88.0 34.0 (struct) (struct :`G` 0.839374 :`B` 1.0 :`A` 1.0))
  (if (`|EnumEquality` (`self.State`) "NewEnumerator6")
    (`SceneComponent.K2_SetWorldLocation` _capsulecomponent (`KismetMathLibrary.MakeVector` _returnvalue_x _returnvalue_y _returnvalue_z) false false))
  (if (`self.ShowABar`)
    (`WidgetComponent.SetTickMode` _awarenessbar "Enabled")
    (else
      (`WidgetComponent.SetTickMode` _awarenessbar "Disabled")))
  (`KismetSystemLibrary.CapsuleTraceSingle` :`Start` _returnvalue :`End` (+ (`KismetMathLibrary.MakeVector` (.x _returnvalue) (.y _returnvalue) (.z _returnvalue)) (`KismetMathLibrary.MakeVector` (* _returnvalue_x_3 1200.0) (* _returnvalue_y_3 1200.0) _returnvalue_z_2)) :`Radius` 20.0 :`HalfHeight` 10.0 :`TraceChannel` "TraceTypeQuery1" :`DrawDebugType` "ForOneFrame"))

(event `self.ReceiveBeginPlay`
  (`SceneComponent.SetVisibility` (`self.SpotLight`) true false)
  (bind _asawareness_bar (cast `/Game/Resources/UI/AwarenessBar` (`WidgetComponent.GetUserWidgetObject` (`self.AwarenessBar`))))
  (set `/Game/Resources/UI/AwarenessBar.Enemy` self _asawareness_bar))

(event `self.ReceiveActorBeginOverlap`
  (params (OtherActor :type "Actor Object Reference"))
  (bind _returnvalue (`self.K2_GetActorLocation`))
  (bind (_returnvalue_x _returnvalue_y) (`KismetMathLibrary.BreakVector` (`KismetMathLibrary.Normal` (- _returnvalue (`SceneComponent.K2_GetComponentLocation` (`Actor.RootComponent` (`self.Other Actor`)))))))
  (set `self.Other Actor` OtherActor)
  (cast `/Game/MyBP/Skill/skills/fairBall` (`self.Other Actor`))
  (`Timeline|Timeline_0` :!label _label
    (:`Update`
      (`SceneComponent.K2_SetWorldLocation` (`self.CapsuleComponent`) (+ _returnvalue (* (`KismetMathLibrary.MakeVector` _returnvalue_x _returnvalue_y) (`self.被火球击退的距离`))) false false))
    (:`Finished`
      (set `self.Other Actor` null)
      (goto _label :!via `SetNewTime`))))

(event `On State Changed`
  (bind _state (`self.State`))
  (`BlackboardComponent.SetValueAsEnum` (`AIBlueprintHelperLibrary.GetBlackboard` null) "State" _state)
  (`KismetSystemLibrary.PrintString` (`|GetEnumeratorNameAsString` _state) true true (struct :`R` 1.0 :`B` 0.96036 :`A` 1.0) 5.0))

(event `/Game/Resources/Blueprints/NPC/Inform.OnFaintActivated`
  (if (`self.Immobile`)
    (set `self.State` "NewEnumerator8")
    (`self.On State Changed`)
    (else
      (set `self.State` "NewEnumerator6")
      (`self.On State Changed`))))

(event `/Game/Resources/Blueprints/NPC/Inform.Blind`
  (set `self.State` "NewEnumerator5")
  (`self.On State Changed`))

(event `ClearAwareness`
  (`BlackboardComponent.SetValueAsFloat` (`AIBlueprintHelperLibrary.GetBlackboard` null) "Awareness" 0.0))

(fn `Faint`
  (bind _mesh (`self.Mesh`))
  (bind _returnvalue (`SceneComponent.K2_GetComponentToWorld` (`self.CapsuleComponent`)))
  ;[1 1 1] 前面设置的那两个变量，可以不用设置，因为用不到了。
  (if (not (`self.Fainting`))
    (set `self.Fainting` true)
    (set `self.LocationBeforeFainted` (`KismetMathLibrary.InverseTransformLocation` _returnvalue (`SceneComponent.K2_GetComponentLocation` _mesh)))
    (set `self.RotationBeforeFainted` (`KismetMathLibrary.InverseTransformRotation` _returnvalue (`SceneComponent.K2_GetComponentRotation` _mesh)))
    (`PrimitiveComponent.SetSimulatePhysics` _mesh true)
    (`CharacterMovementComponent.DisableMovement` (`self.CharacterMovement`))
    (set `self.Immobile` true)))

(fn `Revive`
  (bind _mesh (`self.Mesh`))
  (set `self.Fainting` false)
  (`PrimitiveComponent.SetSimulatePhysics` (`self.Mesh`) false)
  (`SceneComponent.K2_AttachToComponent` _mesh (`self.CapsuleComponent`) "None" "KeepRelative" "KeepRelative" "KeepRelative" true)
  (`SceneComponent.K2_SetRelativeLocationAndRotation` _mesh (0.0 0.0 -90.0) (struct :`Yaw` -90.0) false false)
  (`CharacterMovementComponent.SetMovementMode` (`self.CharacterMovement`) "MOVE_Walking" 0)
  (set `self.Immobile` false))

(fn `UserConstructionScript`)