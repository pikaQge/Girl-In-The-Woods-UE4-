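; Behavior tree task that turns a Knight NPC toward a target location stored in the blackboard.
; On execute it computes the look-at yaw from the actor to that location, discarding pitch and roll.
; It blends the capsule's world rotation 20% toward that yaw along the shortest path, then immediately finishes successfully, so each run makes one partial turn.
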(event `self.ReceiveExecuteAI`
  (params (OwnerController :type "AIController Object Reference") (ControlledPawn :type "Pawn Object Reference"))
  (bind _asknight (cast `/Game/Resources/Blueprints/NPC/Knight` ControlledPawn))
  (bind _capsulecomponent (`Character.CapsuleComponent` _asknight))
  (`SceneComponent.K2_SetWorldRotation` _capsulecomponent (`KismetMathLibrary.RLerp` (`SceneComponent.K2_GetComponentRotation` _capsulecomponent) (`KismetMathLibrary.MakeRotator` 0.0 0.0 (.yaw (`KismetMathLibrary.FindLookAtRotation` (`Actor.K2_GetActorLocation` _asknight) (`BTFunctionLibrary.GetBlackboardValueAsVector` (`self.TargetLocation`))))) 0.2 true) false false)
  (`self.FinishExecute` true))